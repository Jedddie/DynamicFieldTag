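; Builds a hexagonal arena of instanced pillars, sets the player HUD and runs a team score timer.
; Seeded 2D simplex noise splits pillars into static and moving, inside five rising static outer rings.
; Tick time-slices 3D-noise height targets across sections and lerps moving pillars every other frame.
; Authority sets seed and clock, and periodically increments only the first Score entry, once per non-chasing team.
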(event `self.ReceiveBeginPlay`
  (bind _ringcount (`self.RingCount`))
  (`/Engine/EditorBlueprintResources/ActorMacros.Switch Has Authority`
    (:`Authority`
      (set `self.seed` (`KismetMathLibrary.RandomInteger` 0))
      (`KismetArrayLibrary.Array_Resize` (`self.score`) (`self.numTeams`)))
    (:`Remote`
      _))
  (set `self.staticPillarRandomStream` (`KismetMathLibrary.MakeRandomStream` (`self.seed`)))
  (`self.AddPillar` 0)
  (for _index (range 1 (+ _ringcount 1))
    (for _index_2 (range _index)
      (for _index_3 (range 6)
        (`self.AddPillar` _index _index_3 _index_2))))
  (for _index_4 (range (+ _ringcount 1) (+ (+ _ringcount 5) 1))
    (for _index_5 (range _index_4)
      (for _index_6 (range 6)
        (`self.AddPillarStatic` _index_4 _index_6 _index_5 (+ (* (- _index_4 _ringcount) 1000.0) (`KismetMathLibrary.RandomFloatInRangeFromStream` -100.0 100.0 (`self.staticPillarRandomStream`)))))))
  (`/Engine/EditorBlueprintResources/ActorMacros.Switch Has Authority`
    (:`Authority`
      (`KismetSystemLibrary.K2_SetTimerDelegate` (delegate `tick score`) 5.0 true))
    (:`Remote`
      _))
  (`PlayerController.ClientSetHUD` (`GameplayStatics.GetPlayerController` 0) "/Game/UI/PlayerHud/PlayerHud.PlayerHud_C"))

(event `self.ReceiveTick`
  (params (DeltaSeconds :type "Float (single-precision)"))
  (`self.UpdatePillarHeights`)
  (`/Engine/EditorBlueprintResources/StandardMacros.FlipFlop`
    (:`A`
      (`self.lerpPillars` DeltaSeconds))
    (:`B`
      _))
  (`/Engine/EditorBlueprintResources/ActorMacros.Switch Has Authority`
    (:`Authority`
      (set `self.currentTime` (`GameplayStatics.GetTimeSeconds`)))))

(event `tick score`
  (bind _score (`self.score`))
  (for (_ _array_index) _score
    (if (!= _array_index (`self.chasingTeam`))
      (`/Engine/EditorBlueprintResources/StandardMacros.IncrementInt` (`|GetArrayItem` _score)))))

(fn `AddPillar`
  (params (Ring :type Integer) (Face :type Integer) (Index :type Integer))
  (locals (`Pillar Spacing` :type "Float (double-precision)" :default 180.0))
  (bind _returnvalue (* Face 60.0))
  (bind _pillar_spacing (`local.Pillar Spacing`))
  (bind _returnvalue_2 (* (- Face 2) 60.0))
  (bind _returnvalue_3 (+ (* Ring (* (`KismetMathLibrary.DegSin` _returnvalue) _pillar_spacing)) (* Index (* (`KismetMathLibrary.DegSin` _returnvalue_2) _pillar_spacing))))
  (bind _returnvalue_4 (+ (* Ring (* (`KismetMathLibrary.DegCos` _returnvalue) _pillar_spacing)) (* Index (* (`KismetMathLibrary.DegCos` _returnvalue_2) _pillar_spacing))))
  (bind _returnvalue_5 (`KismetSystemLibrary.MakeLiteralBool` (> (`NoiseBlueprintFunctionLibrary.GetSimplex2D` (`self.seed`) 0.0007 _returnvalue_3 _returnvalue_4) 0.55)))
  (`InstancedStaticMeshComponent.AddInstance` (select `bool` _returnvalue_5 :`false` (`self.Pillars`) :`true` (`self.StaticPillars`)) (`KismetMathLibrary.MakeTransform` (`KismetMathLibrary.MakeVector` _returnvalue_3 _returnvalue_4 (select `bool` _returnvalue_5 :`true` (`KismetMathLibrary.RandomFloatInRangeFromStream` 300.0 500.0 (`self.staticPillarRandomStream`))))))
  (if (not _returnvalue_5)
    (`KismetArrayLibrary.Array_Add` (`self.TargetHeights`))
    (`KismetArrayLibrary.Array_Add` (`self.OldHeights`)))
  (return))

(fn `AddPillarStatic`
  (params (Ring :type Integer) (Face :type Integer) (Index :type Integer) (Height :type "Float (double-precision)"))
  (locals (`Pillar Spacing` :type "Float (double-precision)" :default 180.0))
  (bind _returnvalue (* Face 60.0))
  (bind _pillar_spacing (`local.Pillar Spacing`))
  (bind _returnvalue_2 (* (- Face 2) 60.0))
  (`InstancedStaticMeshComponent.AddInstance` (`self.StaticPillars`) (`KismetMathLibrary.MakeTransform` (`KismetMathLibrary.MakeVector` (+ (* Ring (* (`KismetMathLibrary.DegSin` _returnvalue) _pillar_spacing)) (* Index (* (`KismetMathLibrary.DegSin` _returnvalue_2) _pillar_spacing))) (+ (* Ring (* (`KismetMathLibrary.DegCos` _returnvalue) _pillar_spacing)) (* Index (* (`KismetMathLibrary.DegCos` _returnvalue_2) _pillar_spacing))) Height) (struct) (1.2 1.2 1.2)))
  (return))

(fn `lerpPillars`
  (params (`Delta Time` :type "Float (double-precision)"))
  (bind _pillars (`self.Pillars`))
  (for _index (range (`InstancedStaticMeshComponent.GetInstanceCount` _pillars))
    (bind _outinstancetransform (`InstancedStaticMeshComponent.GetInstanceTransform` _pillars _index true))
    (bind _output (`|GetArrayItem` (`self.OldHeights`) _index))
    (bind _output_2 (`|GetArrayItem` (`self.TargetHeights`) _index))
    (`InstancedStaticMeshComponent.UpdateInstanceTransform` _pillars _index (`KismetMathLibrary.MakeTransform` (`KismetMathLibrary.MakeVector` (.x (.location _outinstancetransform)) (.y (.location _outinstancetransform)) (`KismetMathLibrary.Lerp` _output _output_2 (+ (/ (- (.z (.location _outinstancetransform)) _output) (- _output_2 _output)) `Delta Time`))) (.rotation _outinstancetransform) (.scale _outinstancetransform)) true true false))
  (return))

(fn `UpdatePillarHeights`
  (bind _pillars (`self.Pillars`))
  (bind _sectioncount (`self.sectionCount`))
  (bind _returnvalue (`KismetMathLibrary.Conv_IntToDouble` _sectioncount))
  (bind _returnvalue_2 (* (`self.currentTime`) 50.0))
  (bind _returnvalue_3 (/ (`KismetMathLibrary.Conv_IntToDouble` (- (`InstancedStaticMeshComponent.GetInstanceCount` _pillars) 1)) _returnvalue))
  (bind _output_get (set `self.currentSection` (mod (+ (`self.currentSection`) 1) (`self.sectionCount`))))
  (for _index (range (+ (+ (`KismetMathLibrary.FTrunc` _returnvalue_3) (`KismetMathLibrary.FTrunc` (/ (* (`KismetMathLibrary.Fraction` _returnvalue_3) _returnvalue) (`KismetMathLibrary.Conv_IntToDouble` _output_get)))) 1))
    (bind _returnvalue_4 (+ (* _index _sectioncount) _output_get))
    (bind _outinstancetransform (`InstancedStaticMeshComponent.GetInstanceTransform` _pillars _returnvalue_4 true))
    (`KismetArrayLibrary.Array_Set` (`self.TargetHeights`) _returnvalue_4 (* (`NoiseBlueprintFunctionLibrary.GetSimplex3D` (`self.seed`) 0.0005 (+ (.x (.location _outinstancetransform)) _returnvalue_2) (+ (.y (.location _outinstancetransform)) _returnvalue_2) _returnvalue_2) 500.0))
    (`KismetArrayLibrary.Array_Set` (`self.OldHeights`) _returnvalue_4 (.z (.location _outinstancetransform))))
  (return))

(fn `UserConstructionScript`)